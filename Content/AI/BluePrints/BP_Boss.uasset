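; Boss AI character that chases an assigned player target and can show a lock-on marker.
; SetPlayerTarget enters combat and enables Tick, which issues AIMoveTo toward the target; ChasePlayer yaws the boss to face it.
; Chasing and Roaming graphs package similar chase logic and random-point wandering, using a state-driven walk speed helper.
; Lockon flip-flops sphere visibility, and DistanceToPlayer records a pawn line-trace distance.
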(event `/Game/AI/BluePrints/INT_Boss.SetPlayerTarget`
  (params (Target :type "Actor Object Reference"))
  (set `self.PlayerTarget` Target)
  (set `self.isCombat` true)
  (`self.SetActorTickEnabled` true)
  (set `self.StartCombatLocation` (`self.K2_GetActorLocation`)))

(event `/Game/AI/BluePrints/INT_Boss.ChasePlayer`
  (bind (_returnvalue_roll _returnvalue_pitch _returnvalue_yaw) (`KismetMathLibrary.BreakRotator` (`KismetMathLibrary.FindLookAtRotation` (`self.K2_GetActorLocation`) (`self.K2_GetActorLocation` (`self.PlayerTarget`)))))
  (if (`self.isCombat`)
    (`self.PlayerTarget`
      (:`then`
        (`self.K2_SetActorRotation` (`KismetMathLibrary.MakeRotator` 0.0 0.0 _returnvalue_yaw)))
      (:`else`))))

(event `self.ReceiveTick`
  (params (DeltaSeconds :type "Float (single-precision)"))
  (if (`self.isCombat`)
    (`|AIMoveTo` self (0.0 0.0 0.0) (`self.PlayerTarget`) 50.0 true)))

(event `/Game/Flamma/Blueprints/Interfaces/LockOnBPI.LockOn`
  (`/Engine/EditorBlueprintResources/StandardMacros.FlipFlop`
    (:`A`
      (`SceneComponent.SetVisibility` (`self.LockOnSphere`) true false))
    (:`B`
      (`SceneComponent.SetVisibility` (`self.LockOnSphere`) false false))))

(fn `DistanceToPlayer`
  (bind _outhit (`KismetSystemLibrary.LineTraceSingleForObjects` (`self.K2_GetActorLocation`) (`KismetMathLibrary.Conv_RotatorToVector` (`self.K2_GetActorRotation` (`GameplayStatics.GetPlayerPawn` 0))) (`|MakeArray` "ObjectTypeQuery3" :!type "EObjectTypeQuery Enum") false (`|MakeArray` self :!type "Actor Object Reference") "None" true (struct :`R` 1.0 :`A` 1.0) (struct :`G` 1.0 :`A` 1.0) 0.1))
  (set `self.PlayerToEnemyDistance` (`.Distance` (`GameplayStatics.BreakHitResult` _outhit)))
  (set `self.CanBeTarget?` true)
  (return))

(fn `f_MovementState`
  (params (State :type "/Game/_Main/E_AiMovementState Enum" :default "NewEnumerator0"))
  (set `CharacterMovementComponent.MaxWalkSpeed` (select `/Game/_Main/E_AiMovementState` State :`NewEnumerator1` (`self.WalkSpeed`) :`NewEnumerator2` (`self.SpeedMultiplier`)) (`self.CharacterMovement`)))

(fn `UserConstructionScript`
  (`parent.UserConstructionScript`))